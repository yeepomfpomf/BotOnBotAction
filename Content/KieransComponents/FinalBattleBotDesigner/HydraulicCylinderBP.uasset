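; Hydraulic cylinder component for the bot designer, a part with a skeletal piston driven by the HydraulicAxis input.
; The axis shifts the linear Y drive target of the "cylinder" physics constraint, clamped between DecompressionLimit and zero, while a decompression force pushes the bone along the static part's up vector.
; Helper functions pick the static or skeletal mesh and expose sockets and attachment transforms.
; BeginPlay caches the constraint and debug-prints socket names.
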(event `/Game/KieransComponents/Components/ConstraintInterface.HydraulicCylinder`
  (params (HydraulicAxis :type "Float (double-precision)"))
  (bind _constraint (`self.Constraint`))
  (bind _staticpart (`self.StaticPart`))
  (bind _outpostarget (`ConstraintInstanceBlueprintLibrary.GetLinearPositionTarget` _constraint))
  (`ConstraintInstanceBlueprintLibrary.SetLinearPositionTarget` _constraint (`KismetMathLibrary.MakeVector` 0.0 (`KismetMathLibrary.FClamp` (+ (.y _outpostarget) HydraulicAxis) (`self.DecompressionLimit`) 0.0)))
  (`PrimitiveComponent.AddForceAtLocation` (`self.SkeletalPart`) (* (`SceneComponent.GetUpVector` _staticpart) (`self.DecompressionForce`)) (`SceneComponent.K2_GetComponentLocation` _staticpart) "cylinder"))

(event `self.ReceiveBeginPlay`
  (bind _mesh_component (`self.Get Mesh`))
  (set `self.MeshComponent` _mesh_component)
  (bind _returnvalue (`SkeletalMeshComponent.GetConstraintByName` (`self.SkeletalPart`) "cylinder" false))
  (set `self.Constraint` _returnvalue)
  (for _array_element (`SceneComponent.GetAllSocketNames` (`self.SkeletalPart`))
    (`KismetSystemLibrary.PrintString` (`KismetStringLibrary.Conv_NameToString` _array_element) true true (struct :`G` 0.66 :`B` 1.0 :`A` 1.0) 1414.0)))

(event `/Game/KieransComponents/FinalBattleBotDesigner/BBDesignerInterface.Change Pivot`
  (params (Value :type Integer))
  (`self.IndexPivot` Value))

(fn `Attached Transform`
  (params (SocketIndex :type Integer))
  (returns (Transform :type "Transform Structure"))
  (bind _meshcomponent (`self.MeshComponent`))
  (bind (_returnvalue_location _returnvalue_rotation) (`KismetMathLibrary.BreakTransform` (`SceneComponent.GetSocketTransform` _meshcomponent (`|GetArrayItem` (`SceneComponent.GetAllSocketNames` _meshcomponent) SocketIndex) "RTS_World")))
  (return (`KismetMathLibrary.MakeTransform` _returnvalue_location (`KismetMathLibrary.MakeRotFromX` (`KismetMathLibrary.NegateVector` (`KismetMathLibrary.GetForwardVector` _returnvalue_rotation))))))

(fn `Get All Socket Transforms`
  (returns (Transforms :type "Array of Transform Structure"))
  (return (`self.AllSocketTransforms`)))

(fn `Get All Sockets`
  (returns (Sockets :type "Array of Name"))
  (return (`self.Sockets`)))

(fn `Get Mesh`
  (returns (`Mesh Component` :type "PrimitiveComponent Object Reference") (Constrain :type Boolean))
  (bind _constrain (`self.Constrain`))
  (if (`self.SM`)
    (return (`self.StaticPart`) _constrain)
    (else
      (return (`self.SkeletalPart`) _constrain))))

(fn `Get Socket By Index`
  (params (Index :type Integer))
  (returns (Socket :type Name))
  (return (`|GetArrayItem` (`self.Sockets`) Index)))

(fn `UserConstructionScript`
  (`parent.UserConstructionScript`))