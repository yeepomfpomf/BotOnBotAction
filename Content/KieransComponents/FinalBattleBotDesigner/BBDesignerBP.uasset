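; Player-controlled battle bot designer that builds a machine from a starting part, then physics-simulates and drives it.
; A spawned hydraulic cylinder snaps to the closest socket under the cursor, and clicking attaches it, adding physics constraints for constrained meshes.
; G starts simulation, after which throttle, steer and hydraulics input reach tagged controlled parts through message calls.
; A/D changes the pending part's pivot, Shift plus mouse rotates the view, and the wheel zooms.
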(event `Key|LeftShift`
  (params (Key :type "Key Structure"))
  (bind _returnvalue (`GameplayStatics.GetPlayerController` 0))
  (:`Pressed`
    (set `self.Holding Shift` true)
    (set `PlayerController.bShowMouseCursor` false _returnvalue))
  (:`Released`
    (set `self.Holding Shift` false)
    (set `PlayerController.bShowMouseCursor` true _returnvalue)))

(event `InputAxis|Throttle`
  (params (AxisValue :type "Float (single-precision)"))
  (for _array_element (`self.ControlledParts`)
    (if (`self.Simulating?`)
      (if (`self.ActorHasTag` _array_element "Wheel")
        (message `/Game/KieransComponents/Components/ConstraintInterface.Throttle` _array_element AxisValue)))))

(event `Key|A`
  (params (Key :type "Key Structure"))
  (:`Pressed`
    (message `/Game/KieransComponents/FinalBattleBotDesigner/BBDesignerInterface.Change Pivot` (`self.Child`) -1)))

(event `EnhancedInput|/Game/KieransComponents/FinalBattleBotDesigner/Inputs/BBDesignerMouse`
  (params (ActionValue :type "Vector2D Structure") (ElapsedSeconds :type "Float (double-precision)") (TriggeredSeconds :type "Float (double-precision)") (InputAction :type "InputAction Object Reference" :default "/Game/KieransComponents/FinalBattleBotDesigner/Inputs/BBDesignerMouse.BBDesignerMouse"))
  (:`Triggered`
    (if (`self.Holding Shift`)
      (`self.AddControllerYawInput` ActionValue_X)
      (`self.AddControllerPitchInput` ActionValue_Y))))

(event `InputAxis|Steer`
  (params (AxisValue :type "Float (single-precision)"))
  (for _array_element (`self.ControlledParts`)
    (if (`self.Simulating?`)
      (if (`self.ActorHasTag` _array_element "Wheel")
        (message `/Game/KieransComponents/Components/ConstraintInterface.Steer` _array_element AxisValue)))))

(event `Key|D`
  (params (Key :type "Key Structure"))
  (:`Pressed`
    (message `/Game/KieransComponents/FinalBattleBotDesigner/BBDesignerInterface.Change Pivot` (`self.Child`) 1)))

(event `InputAxisKey|MouseWheelAxis`
  (params (AxisValue :type "Float (single-precision)"))
  (bind _springarm (`self.SpringArm`))
  (set `SpringArmComponent.TargetArmLength` (+ (`SpringArmComponent.TargetArmLength` _springarm) (* AxisValue 30.0 -1.0)) _springarm))

(event `InputAxis|Hydraulics`
  (params (AxisValue :type "Float (single-precision)"))
  (if (`self.Simulating?`)
    (for _array_element (`self.ControlledParts`)
      (if (`self.ActorHasTag` _array_element "Hydraulic")
        (message `/Game/KieransComponents/Components/ConstraintInterface.HydraulicCylinder` _array_element AxisValue)))))

(event `self.ReceiveBeginPlay`
  (`EnhancedInputSubsystemInterface.AddMappingContext` (pcsubsystem `EnhancedInputLocalPlayerSubsystem` (`GameplayStatics.GetPlayerController` 0)) "/Game/KieransComponents/FinalBattleBotDesigner/Inputs/BBDesignerIMC.BBDesignerIMC" 0 (struct))
  (bind _returnvalue (`|SpawnActorFromClass` "/Game/KieransComponents/FinalBattleBotDesigner/PartBP.PartBP_C" (`self.GetTransform`) "Undefined" "MultiplyWithRoot" null null))
  (`PrimitiveComponent.SetCollisionResponseToChannel` (`/Game/KieransComponents/FinalBattleBotDesigner/PartBP.StaticPart` _returnvalue) "ECC_Visibility" "ECR_Block")
  (bind _output_get (set `self.FirstPart` _returnvalue))
  (set `self.Parent` _output_get))

(event `Key|F`
  (params (Key :type "Key Structure"))
  (:`Pressed`
    (bind _returnvalue (`|SpawnActorFromClass` "/Game/KieransComponents/FinalBattleBotDesigner/HydraulicCylinderBP.HydraulicCylinderBP_C" (`KismetMathLibrary.MakeTransform` (0.0 0.0 10000.0)) "Undefined" "MultiplyWithRoot" null null))
    (set `self.Child` _returnvalue)))

(event `EnhancedInput|/Game/KieransComponents/FinalBattleBotDesigner/Inputs/BBDesignerMouse`
  (params (ActionValue :type "Vector2D Structure") (ElapsedSeconds :type "Float (double-precision)") (TriggeredSeconds :type "Float (double-precision)") (InputAction :type "InputAction Object Reference" :default "/Game/KieransComponents/FinalBattleBotDesigner/Inputs/BBDesignerMouse.BBDesignerMouse"))
  (bind (_impactpoint _hitactor _returnvalue) (`self.GetCursorHit`))
  (:`Triggered`
    (if (not (`self.Holding Shift`))
      (`/Engine/EditorBlueprintResources/StandardMacros.IsValid` (`self.Child`)
        (:`Is Valid`
          (if _returnvalue
            (bind _output_get (set `self.Parent` _hitactor))
            (bind _transforms (message `/Game/KieransComponents/FinalBattleBotDesigner/BBDesignerInterface.Get All Socket Transforms` _output_get))
            (bind _socketindex (`self.GetClosestSocket` _impactpoint _transforms))
            (bind _output_get_2 (set `self.Socket Index` _socketindex))
            (bind _transform (message `/Game/KieransComponents/FinalBattleBotDesigner/BBDesignerInterface.Attached Transform` (`self.Parent`) _output_get_2))
            (bind _output_get_3 (set `self.AttachedTransform` _transform))
            (`self.K2_SetActorTransform` (`self.Child`) (`KismetMathLibrary.MakeTransform` (.location _output_get_3) (.rotation _output_get_3)) false false)))))))

(event `Key|LeftMouseButton`
  (params (Key :type "Key Structure"))
  (:`Pressed`
    (bind (_mesh_component _constrain) (message `/Game/KieransComponents/FinalBattleBotDesigner/BBDesignerInterface.Get Mesh` (`self.Parent`)))
    (set `self.ParentMeshComponenet` _mesh_component)
    (set `self.ParentMeshIsConstrained` _constrain)
    (bind (_mesh_component_2 _constrain_2) (message `/Game/KieransComponents/FinalBattleBotDesigner/BBDesignerInterface.Get Mesh` (`self.Child`)))
    (set `self.ChildMeshComponent` _mesh_component_2)
    (set `self.ChildMeshConstrained` _constrain_2)
    (`self.K2_AttachToComponent` (`self.Child`) (`self.ParentMeshComponenet`) (`|GetArrayItem` (`SceneComponent.GetAllSocketNames` (`self.ParentMeshComponenet`)) (`self.Socket Index`)) "KeepWorld" "KeepWorld" "KeepWorld" true)
    (if (or (`self.ParentMeshIsConstrained`) (`self.ChildMeshConstrained`))
      (`self.Handle Constrained Components` (`self.ChildMeshComponent`))
      (`KismetArrayLibrary.Array_Add` (`self.ControlledParts`) (`self.Child`))
      (set `self.Child` null))))

(event `Key|G`
  (params (Key :type "Key Structure"))
  (bind _parentmeshcomponenet (`self.ParentMeshComponenet`))
  (:`Pressed`
    (`PrimitiveComponent.SetSimulatePhysics` _parentmeshcomponenet true)
    (set `self.Simulating?` true)
    (`SceneComponent.K2_AttachToComponent` (`self.SpringArm`) _parentmeshcomponenet "None" "KeepWorld" "KeepWorld" "KeepWorld" true)))

(fn `Attached Transform`
  (params (SocketIndex :type Integer))
  (returns (Transform :type "Transform Structure"))
  (return))

(fn `Correct Mouse`)

(fn `Create Constraint`
  (params (`Constraint Transform` :type "Transform Structure") (Component1 :type Name) (Component2 :type Name))
  (bind _returnvalue (`AddComponent|NODE_AddPhysicsConstraintComponent-4` :`RelativeTransform` `Constraint Transform`))
  (`PhysicsConstraintComponent.SetConstrainedComponents` _returnvalue (`self.ParentMeshComponenet`) Component1 (`self.ChildMeshComponent`) Component2))

(fn `Get All Socket Transforms`
  (returns (Transforms :type "Array of Transform Structure"))
  (return))

(fn `Get All Sockets`
  (returns (Sockets :type "Array of Name"))
  (return))

(fn `Get Mesh`
  (returns (`Mesh Component` :type "PrimitiveComponent Object Reference") (Constrain :type Boolean))
  (return null false))

(fn `Get Socket By Index`
  (params (Index :type Integer))
  (returns (Socket :type Name))
  (return "None"))

(fn `GetClosestSocket`
  (params (`Impact Point` :type "Vector Structure") (Transforms :type "Array of Transform Structure"))
  (returns (SocketIndex :type Integer))
  (locals (Distance :type "Float (double-precision)" :default 6942069.0))
  (for (_array_element _array_index) Transforms
    (bind _returnvalue (`KismetMathLibrary.Vector_Distance` `Impact Point` (.location _array_element)))
    (if (< _returnvalue (`local.Distance`))
      (set `self.Socket Index` _array_index)
      (set `local.Distance` _returnvalue)))
  (return (`self.Socket Index`)))

(fn `GetCursorHit`
  (returns (ImpactPoint :type "Vector Structure") (HitActor :type "Actor Object Reference") (ReturnValue :type Boolean) (Rotation :type "Rotator Structure"))
  (bind _returnvalue (`GameplayStatics.GetPlayerController` 0))
  (bind (_locationx _locationy) (`PlayerController.GetMousePosition` _returnvalue))
  (bind (_bblockinghit _binitialoverlap _time _distance _location _impactpoint _normal _impactnormal _physmat _hitactor) (`GameplayStatics.BreakHitResult` (`PlayerController.GetHitResultUnderCursorByChannel` _returnvalue "TraceTypeQuery1" true)))
  (`PlayerController.SetMouseLocation` _returnvalue (`KismetMathLibrary.FTrunc` _locationx) (`KismetMathLibrary.FTrunc` _locationy))
  (return _impactpoint _hitactor _bblockinghit (`KismetMathLibrary.MakeRotFromX` _normal)))

(fn `Handle Constrained Components`
  (params (Mesh :type "PrimitiveComponent Object Reference"))
  (bind _childmeshconstrained (`self.ChildMeshConstrained`))
  (bind _socket (message `/Game/KieransComponents/FinalBattleBotDesigner/BBDesignerInterface.Get Socket By Index` (`self.Parent`) (`self.Socket Index`)))
  (if (`self.ParentMeshIsConstrained`)
    (if _childmeshconstrained
      (bind _returnvalue (`SceneComponent.GetSocketTransform` (`self.ParentMeshComponenet`) _socket "RTS_Actor"))
      (`self.Create Constraint` _returnvalue "top" "bottom")
      (else
        (`self.Create Constraint` _returnvalue "bottom")))
    (`PrimitiveComponent.SetCollisionResponseToAllChannels` Mesh "ECR_Block" :!label _label)
    (`PrimitiveComponent.SetSimulatePhysics` Mesh true)
    (return)
    (elif _childmeshconstrained
      (`self.Create Constraint` _returnvalue "None" "bottom")
      (goto _label))))

(fn `UserConstructionScript`)