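; Base part for a bot designer, wrapping either a static or skeletal mesh whose sockets act as pivot and attachment points.
; On BeginPlay it caches the socket names and world transforms.
; ChangePivot cycles through sockets with wraparound, offsetting the mesh and counter-rotating the Pivot so the chosen socket becomes the origin.
; AttachedTransform gives a socket's world location facing against its forward axis, and getters expose the mesh and socket data.
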(event `self.ReceiveBeginPlay`
  (bind _mesh (`self.Get Mesh Component`))
  (bind _output_get (set `self.MeshComponent` _mesh))
  (set `self.Sockets` (`SceneComponent.GetAllSocketNames` _output_get))
  (`self.IndexPivot` 0)
  (for _array_element (`self.Sockets`)
    (`KismetArrayLibrary.Array_Add` (`self.AllSocketTransforms`) (`SceneComponent.GetSocketTransform` _output_get _array_element "RTS_World"))))

(event `/Game/KieransComponents/FinalBattleBotDesigner/BBDesignerInterface.Change Pivot`
  (params (Value :type Integer))
  (`self.IndexPivot` Value))

(fn `Attached Transform`
  (params (SocketIndex :type Integer))
  (returns (Transform :type "Transform Structure"))
  (bind _meshcomponent (`self.MeshComponent`))
  (bind (_returnvalue_location _returnvalue_rotation) (`KismetMathLibrary.BreakTransform` (`SceneComponent.GetSocketTransform` _meshcomponent (`|GetArrayItem` (`SceneComponent.GetAllSocketNames` _meshcomponent) SocketIndex) "RTS_World")))
  (return (`KismetMathLibrary.MakeTransform` _returnvalue_location (`KismetMathLibrary.MakeRotFromX` (`KismetMathLibrary.NegateVector` (`KismetMathLibrary.GetForwardVector` _returnvalue_rotation))))))

(fn `Get All Socket Transforms`
  (returns (Transforms :type "Array of Transform Structure"))
  (return (`self.AllSocketTransforms`)))

(fn `Get All Sockets`
  (returns (Sockets :type "Array of Name"))
  (return (`self.Sockets`)))

(fn `Get Mesh`
  (returns (`Mesh Component` :type "PrimitiveComponent Object Reference") (Constrain :type Boolean))
  (return (`self.MeshComponent`) (`self.Constrain`)))

(fn `Get Mesh Component`
  (returns (Mesh :type "PrimitiveComponent Object Reference"))
  (if (`self.SM`)
    (return (`self.StaticPart`))
    (else
      (return (`self.SkeletalPart`)))))

(fn `Get Socket By Index`
  (params (Index :type Integer))
  (returns (Socket :type Name))
  (return (`|GetArrayItem` (`self.Sockets`) Index)))

(fn `IndexPivot`
  (params (Index :type Integer))
  (bind _sockets (`self.Sockets`))
  (bind _meshcomponent (`self.MeshComponent`))
  (bind _returnvalue (`KismetArrayLibrary.Array_Length` _sockets))
  (bind _output_get (set `self.Pivot Point` (mod (+ Index (`self.Pivot Point`) _returnvalue) _returnvalue)))
  (bind (_returnvalue_location _returnvalue_rotation) (`KismetMathLibrary.BreakTransform` (`SceneComponent.GetSocketTransform` _meshcomponent (`|GetArrayItem` _sockets _output_get) "RTS_Component")))
  (`SceneComponent.K2_SetRelativeLocation` _meshcomponent (* _returnvalue_location -1) false false)
  (`SceneComponent.K2_SetRelativeRotation` (`self.Pivot`) (`KismetMathLibrary.NegateRotator` _returnvalue_rotation) false false))

(fn `UserConstructionScript`)