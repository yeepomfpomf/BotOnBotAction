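; Physics-driven wheel Blueprint that turns throttle and steer input into torque around the static mesh's right axis.
; Throttle torque flips sign for left versus right wheels, while steering adds mass-independent torque with no side flip.
; On BeginPlay it spawns and attaches a WheelEffects actor for skids and sound, fed speed, RPM and roll.
; Helper functions expose the mesh, constraint, sockets and attach transforms.
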(event `/Game/KieransComponents/Components/ConstraintInterface.Throttle`
  (params (ThrottleAxis :type "Float (double-precision)"))
  ;[1 1 1] Comment
  (`self.WheelThrottle` ThrottleAxis)
  (`KismetSystemLibrary.PrintString` "Hello"))

(event `/Game/KieransComponents/Components/ConstraintInterface.Steer`
  (params (SteerAxis :type "Float (double-precision)"))
  ;[1 1 1] Comment
  (`self.WheelSteer` SteerAxis))

(event `self.ReceiveTick`
  (params (DeltaSeconds :type "Float (single-precision)"))
  (bind _returnvalue_roll (`KismetMathLibrary.BreakRotator` (`SceneComponent.K2_GetComponentRotation` (`self.StaticPart`))))
  ;[1 1 1] Sets Skid And Sound Effects
  (`/Game/Wheels/WheelEffects.SkidMarkCorrection` (`self.WheelEffectReference`) (`KismetMathLibrary.Abs` _returnvalue_roll))
  (bind _rpm (`/Game/KieransComponents/FunctionLibrary/KieransComponentLibrary.Get RPM` null (`self.StaticPart`)))
  (set `self.RPM` _rpm))

(event `self.ReceiveBeginPlay`
  (`self.Intialisesoundandskid`))

(event `/Game/KieransComponents/FinalBattleBotDesigner/BBDesignerInterface.Change Pivot`
  (params (Value :type Integer))
  (`self.IndexPivot` Value))

(fn `Attached Transform`
  (params (SocketIndex :type Integer))
  (returns (Transform :type "Transform Structure"))
  (bind _meshcomponent (`self.MeshComponent`))
  (bind (_returnvalue_location _returnvalue_rotation) (`KismetMathLibrary.BreakTransform` (`SceneComponent.GetSocketTransform` _meshcomponent (`|GetArrayItem` (`SceneComponent.GetAllSocketNames` _meshcomponent) SocketIndex) "RTS_World")))
  (return (`KismetMathLibrary.MakeTransform` _returnvalue_location (`KismetMathLibrary.MakeRotFromX` (`KismetMathLibrary.NegateVector` (`KismetMathLibrary.GetForwardVector` _returnvalue_rotation))))))

(fn `Get All Socket Transforms`
  (returns (Transforms :type "Array of Transform Structure"))
  (return (`self.AllSocketTransforms`)))

(fn `Get All Sockets`
  (returns (Sockets :type "Array of Name"))
  (return (`self.Sockets`)))

(fn `Get Mesh`
  (returns (`Mesh Component` :type "PrimitiveComponent Object Reference") (Constrain :type Boolean))
  (bind _constrain (`self.Constrain`))
  (if (`self.SM`)
    (return (`self.StaticPart`) _constrain)
    (else
      (return (`self.SkeletalPart`) _constrain))))

(fn `Get Socket By Index`
  (params (Index :type Integer))
  (returns (Socket :type Name))
  (return (`|GetArrayItem` (`self.Sockets`) Index)))

(fn `Intialisesoundandskid`
  (bind _returnvalue (`|SpawnActorFromClass` "/Game/Wheels/WheelEffects.WheelEffects_C" (`KismetMathLibrary.MakeTransform` (0.0 0.0 0.0)) "AlwaysSpawn" "MultiplyWithRoot" null null))
  (set `self.WheelEffectReference` _returnvalue)
  (`self.K2_AttachToComponent` _returnvalue (`self.StaticPart`) "None" "KeepRelative" "KeepRelative" "KeepRelative" true)
  (`/Game/Wheels/WheelEffects.InitaliseEffects` (`self.WheelEffectReference`)))

(fn `UserConstructionScript`
  (`parent.UserConstructionScript`))

(fn `WheelSteer`
  (params (A :type "Float (single-precision)"))
  (locals (TurnDirection :type "Float (double-precision)"))
  (bind _staticpart (`self.StaticPart`))
  (set `self.steeraxis` A)
  (if (!= A 0.0)
    (set `self.Cancel Throttle` 0.0)
    (else
      (set `self.Cancel Throttle` 1.0)))
  (`PrimitiveComponent.AddTorqueInDegrees` _staticpart (* (* A (`self.SteerTorque`)) (`SceneComponent.GetRightVector` _staticpart)) "None" true)
  (return))

(fn `WheelThrottle`
  (params (A :type "Float (single-precision)"))
  (bind _staticpart (`self.StaticPart`))
  (set `self.ThrottleAxis` A)
  (`|ExecutionSequence`
    (:`then_0`
      (if (`self.RightWheels`)
        (set `self.TurnDirection` 1.0)
        (else
          (set `self.TurnDirection` -1.0))))
    (:`then_1`
      (`PrimitiveComponent.AddTorqueInRadians` _staticpart (* (* A (`self.Torque`) (`self.TurnDirection`)) (`SceneComponent.GetRightVector` _staticpart)) "None" false)
      (bind _output_get (set `self.Speed` (`KismetMathLibrary.VSize` (`SceneComponent.GetComponentVelocity` _staticpart))))
      (`/Game/Wheels/WheelEffects.Throttle` (`self.WheelEffectReference`) 0.0 _output_get (`self.RPM`))
      (return))))