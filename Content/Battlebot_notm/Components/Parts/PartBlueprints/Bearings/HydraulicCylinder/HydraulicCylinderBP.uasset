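; Battlebot hydraulic cylinder part whose extension is driven by the HydraulicCylinder input axis.
; BeginPlay caches the skeletal part's "cylinder" physics constraint, and each axis event shifts its linear Y position target, clamped between DecompressionLimit and zero.
; The same event also pushes the cylinder bone along the static part's up vector with DecompressionForce, whatever the axis value.
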(event `/Game/KieransComponents/Components/ConstraintInterface.HydraulicCylinder`
  (params (HydraulicAxis :type "Float (double-precision)"))
  (bind _constraint (`self.Constraint`))
  (bind _staticpart (`self.StaticPart`))
  (bind _outpostarget (`ConstraintInstanceBlueprintLibrary.GetLinearPositionTarget` _constraint))
  (`ConstraintInstanceBlueprintLibrary.SetLinearPositionTarget` _constraint (`KismetMathLibrary.MakeVector` 0.0 (`KismetMathLibrary.FClamp` (+ (.y _outpostarget) HydraulicAxis) (`self.DecompressionLimit`) 0.0)))
  (`PrimitiveComponent.AddForceAtLocation` (`self.SkeletalPart`) (* (`SceneComponent.GetUpVector` _staticpart) (`self.DecompressionForce`)) (`SceneComponent.K2_GetComponentLocation` _staticpart) "cylinder"))

(event `self.ReceiveBeginPlay`
  (bind _returnvalue (`SkeletalMeshComponent.GetConstraintByName` (`self.SkeletalPart`) "cylinder" false))
  (set `self.Constraint` _returnvalue))

(fn `UserConstructionScript`
  (`parent.UserConstructionScript`))